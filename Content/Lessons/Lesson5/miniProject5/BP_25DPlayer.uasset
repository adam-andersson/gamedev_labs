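; Player character for a 2.5D game that carries and shoots basketballs while avoiding enemies, with a spawned camera and HUD.
; A physics handle holds a ball picked up from the front box, then drops it or launches it with timeline-driven power.
; Each tick it flags enemies inside its vision volume, alerting them to approach.
; Enemy contact costs health with a brief grace period, and death restarts the level in slow motion.
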(event OnComponentBeginOverlap(DamageHitbox)
  (params (OverlappedComponent :type Primitive%20Component%20Object%20Reference) (OtherActor :type Actor%20Object%20Reference) (OtherComp :type Primitive%20Component%20Object%20Reference) (OtherBodyIndex :type Integer) (bFromSweep :type Boolean) (SweepResult :type Hit%20Result%20Structure%20%28by%20ref%29))
  (bind _mesh (Variables|Character|GetMesh))
  (bind _returnvalue (Transformation|GetWorldLocation _mesh))
  (bind _returnvalue_2 (+ _returnvalue "0,0.000000,90.000000"))
  (Utilities|Casting|CastToBP_Enemy OtherActor)
  (if (Variables|Actor|GetbCanBeDamaged)
    (Effects|SpawnEmitteratLocation "/Game/Effects/Particles/Explosion/P_NeonExplosion.P_NeonExplosion" _returnvalue_2 "0, 0, 0" "0.800000,0.800000,0.800000")
    (Audio|PlaySoundatLocation "/Game/Audio/SoundWaves/Effect/SW_Thud_1.SW_Thud_1" _returnvalue_2 "0, 0, 0" 1.0 1.0 0.0 0 0 0)
    (Variables|Default|SetCurrentHealth (- (Variables|Default|GetCurrentHealth) 2e+01))
    (Variables|Actor|SetbCanBeDamaged false)
    (bind _playerdead (CallFunction|DidPlayerDie))
    (if _playerdead
      (Audio|PlaySoundatLocation "/Game/Audio/SoundWaves/Effect/SW_Explosion_1.SW_Explosion_1" (Transformation|GetActorLocation) "0, 0, 0" 1.0 1.0 0.0 0 0 0)
      (Utilities|Time|SetGlobalTimeDilation 0.1)
      ;[1 1 1] Restart level on death
      (bind _returnvalue_3 (Game|GetCurrentLevelName true))
      (Utilities|FlowControl|Delay 0.5)
      (Game|OpenLevel(byName) (Utilities|String|StringToName _returnvalue_3))
      (else
        ;[1 1 1] 1 second grace period after taking damage
        (Utilities|FlowControl|Delay 1.0)
        (Variables|Actor|SetbCanBeDamaged true)))))

(event OnComponentBeginOverlap(InFrontBox)
  (params (OverlappedComponent :type Primitive%20Component%20Object%20Reference) (OtherActor :type Actor%20Object%20Reference) (OtherComp :type Primitive%20Component%20Object%20Reference) (OtherBodyIndex :type Integer) (bFromSweep :type Boolean) (SweepResult :type Hit%20Result%20Structure%20%28by%20ref%29))
  (Utilities|Casting|CastToBP_Basketball OtherActor)
  (Variables|Default|SetBallToPickUp OtherComp))

(event OnComponentEndOverlap(InFrontBox)
  (params (OverlappedComponent :type Primitive%20Component%20Object%20Reference) (OtherActor :type Actor%20Object%20Reference) (OtherComp :type Primitive%20Component%20Object%20Reference) (OtherBodyIndex :type Integer))
  (Variables|Default|SetBallToPickUp 0))

(event EventBeginPlay
  (bind _returnvalue (Game|SpawnActorfromClass "/Game/Lessons/Lesson5/miniProject5/BP_25DCamera.BP_25DCamera_C" (Transformation|GetWorldTransform (Variables|Default|GetCameraSpawnPoint)) "Undefined" 0 0))
  (Game|Player|SetViewTargetwithBlend (Game|GetPlayerController 0) _returnvalue 0.0 "VTBlend_Linear" 0.0 false)
  (bind _returnvalue_2 (UserInterface|CreateWidget "/Game/Lessons/Lesson5/miniProject5/HUD.HUD_C"))
  (UserInterface|Viewport|AddtoViewport _returnvalue_2 0)
  (bind _shotpower (Timeline|ShotPowerTimeline Play)
    (:Update
      (Variables|Default|SetCurrentPower (* _shotpower 1e+04)))))

(event EventTick
  (params (DeltaSeconds :type Float%20%28single-precision%29))
  (bind _outactors (Actor|GetAllActorsOfClass "/Game/Lessons/Lesson5/miniProject5/BP_Enemy.BP_Enemy_C"))
  (for _array_element _outactors
    (bind _asbp_enemy (Utilities|Casting|CastToBP_Enemy _array_element))
    (Variables|/Game/Lessons/Lesson5/miniProject5/BP_Enemy.BP_Enemy_C|SetinVision _asbp_enemy false))
  ;[1 1 1] Update position of carried ball
  (Class|PhysicsHandleComponent|SetTargetLocationandRotation (Variables|Default|GetPhysicsHandle) (Transformation|GetWorldLocation (Variables|Default|GetSnapPoint)) "0, 0,0.000000")
  (for _array_element_2 (Collision|GetOverlappingActors (Variables|Default|GetPlayerVision) "/Game/Lessons/Lesson5/miniProject5/BP_Enemy.BP_Enemy_C" :!class /Script/Engine.PrimitiveComponent)
    ;[1 1 1] All enemies that are in player's view get alerted and move towards player
    (bind _asbp_enemy_2 (Utilities|Casting|CastToBP_Enemy _array_element_2))
    (Variables|/Game/Lessons/Lesson5/miniProject5/BP_Enemy.BP_Enemy_C|SetinVision _asbp_enemy_2 true)
    (Variables|/Game/Lessons/Lesson5/miniProject5/BP_Enemy.BP_Enemy_C|SetPlayerForward _asbp_enemy_2 (Math|Vector|GetForwardVector (Variables|Default|GetArrow1)))))

(event Input|ActionEvents|InputActionPrimaryAction
  (params (Key :type Key%20Structure :default "None"))
  (:Pressed
    (if (Variables|Default|GetIsGrabbing)
      (Physics|Components|PhysicsHandle|ReleaseComponent (Variables|Default|GetPhysicsHandle))
      (Variables|Default|SetObjectToMove 0)
      (Variables|Default|SetIsGrabbing false)
      (Rendering|SetVisibility (Variables|Default|GetShootDirection) false false)
      (elif (Utilities|IsValid (Variables|Default|GetBallToPickUp))
        (bind _output_get (Variables|Default|SetObjectToMove (Variables|Default|GetBallToPickUp)))
        (CallFunction|MoveObject _output_get)
        (Rendering|SetVisibility (Variables|Default|GetShootDirection) true false)))))

(event Input|ActionEvents|InputActionSecondaryAction
  (params (Key :type Key%20Structure :default "None"))
  (:Pressed
    (if (Variables|Default|GetIsGrabbing)
      (Physics|Components|PhysicsHandle|ReleaseComponent (Variables|Default|GetPhysicsHandle))
      (Physics|AddImpulse (Variables|Default|GetObjectToMove) (* (Math|Vector|GetForwardVector (Variables|Default|GetShootDirection)) (Variables|Default|GetCurrentPower)) "None" false)
      (Variables|Default|SetIsGrabbing false)
      (Variables|Default|SetObjectToMove 0)
      (Rendering|SetVisibility (Variables|Default|GetShootDirection) false false))))

(event Input|AxisEvents|InputAxisMoveRight
  (params (AxisValue :type Float%20%28single-precision%29))
  (Pawn|Input|AddMovementInput "0,1.000000, 0" AxisValue false))

(event Input|AxisEvents|InputAxisMoveForward
  (params (AxisValue :type Float%20%28single-precision%29))
  (Pawn|Input|AddMovementInput "1.000000, 0, 0" AxisValue false))

(fn ConstructionScript)

(fn MoveObject
  (params (ObjectToMove :type Primitive%20Component%20Object%20Reference))
  (Class|PhysicsHandleComponent|GrabComponentatLocation (Variables|Default|GetPhysicsHandle) ObjectToMove "None" (Transformation|GetWorldLocation ObjectToMove))
  (Variables|Default|SetIsGrabbing true))

(fn DidPlayerDie
  (return (<= (Variables|Default|GetCurrentHealth) 0.0)))