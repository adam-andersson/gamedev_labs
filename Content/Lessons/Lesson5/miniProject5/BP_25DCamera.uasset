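; BP_25DCamera is a 2.5D follow camera that tracks player character 0 along Y and Z while holding a constant X.
; BeginPlay stores the offset from the player and the camera's starting X.
; Tick rebuilds the location from that X and the player's Y and Z, then adds the full offset, so the fixed X includes the initial X offset too.
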(event EventBeginPlay
  (bind _returnvalue (Transformation|GetActorLocation))
  (Variables|Default|SetCamera%20Offset (- _returnvalue (Transformation|GetActorLocation (Game|GetPlayerCharacter 0))))
  (Variables|Default|SetCamera%20X%20Location (.X (Math|Vector|BreakVector _returnvalue))))

(event EventTick
  (params (DeltaSeconds :type Float%20%28single-precision%29))
  (bind _returnvalue (Game|GetPlayerCharacter 0))
  (bind _returnvalue_2 (Transformation|GetActorLocation _returnvalue))
  (Transformation|SetActorLocation (+ (Math|Vector|MakeVector (Variables|Default|GetCamera%20X%20Location) (.y _returnvalue_2) (.z _returnvalue_2)) (Variables|Default|GetCamera%20Offset)) false false))

(fn ConstructionScript)