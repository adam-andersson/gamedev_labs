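; BP_Enemy is a lesson mini-project enemy that moves only while it is in vision.
; Each tick HaveBeenSeen checks the InVision flag.
; When set, it applies an impulse to its physics Sphere along the negated PlayerForward vector.
; When clear, it zeroes the sphere's horizontal velocity, passing through only the actor's vertical velocity.
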(event EventTick
  (params (DeltaSeconds :type Float%20%28single-precision%29))
  (CallFunction|HaveBeenSeen))

(fn ConstructionScript)

(fn HaveBeenSeen
  (if (Variables|Default|GetinVision)
    ;[1 1 1] Move towards negation of player's forward vector
    (Physics|AddImpulse (Variables|Default|GetSphere) (* (Math|Vector|NegateVector (Variables|Default|GetPlayerForward)) 3e+02) "None" false)
    (else
      ;[1 1 1] Stop all movement when out of vision, 'Out of sight, out of mind'
      (Physics|SetPhysicsLinearVelocity (Variables|Default|GetSphere) (Math|Vector|MakeVector 0.0 0.0 (.z (Transformation|GetVelocity))) false "None"))))