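; Minecart actor that moves along world Y and sprays wheel sparks as it brakes.
; Each Tick adds a positive Y offset scaled by absolute Y, delta time and UnitsPerDelta, so it eases to a stop when approaching zero from negative Y.
; While at least a threshold distance from Y zero, it spawns small asteroid-explosion emitters at both wheel spark components every frame.
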(event EventBeginPlay)

(event Collision|EventActorBeginOverlap
  (params (OtherActor :type Actor%20Object%20Reference)))

(event EventTick
  (params (DeltaSeconds :type Float%20%28single-precision%29))
  (bind _returnvalue (Transformation|GetActorLocation))
  (bind _returnvalue_2 (Math|Float|Absolute(Float) (.y _returnvalue)))
  ;[1 1 1] Minecart only breaks if it have not fully stopped
  (if (>= _returnvalue_2 1e+02)
    (Effects|SpawnEmitteratLocation "/Game/Effects/Particles/Explosion/P_AsteroidExplosion.P_AsteroidExplosion" (Transformation|GetWorldLocation (Variables|Default|GetLeftWheelSparks)) "0, 0, 0" "0.100000,0.100000,0.100000")
    (Effects|SpawnEmitteratLocation "/Game/Effects/Particles/Explosion/P_AsteroidExplosion.P_AsteroidExplosion" (Transformation|GetWorldLocation (Variables|Default|GetRightWheelSparks)) "0, 0, 0" "0.100000,0.100000,0.100000"))
  (Transformation|AddActorWorldOffset (Math|Vector|MakeVector 0.0 (* (/ _returnvalue_2 3.0) (* DeltaSeconds (Variables|Default|GetUnitsPerDelta))) 0.0)))

(fn ConstructionScript)