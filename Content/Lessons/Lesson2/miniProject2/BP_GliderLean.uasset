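; Glider actor that runs along a runway and takes off on its own in a lesson mini project.
; Each Tick it spawns a small explosion emitter at the engine and moves diagonally in X/Y, at a speed derived from its X position and the runway end.
; Once the mesh's X drops to 1000 or below, it records the lift-off time, then climbs at Speed while time-based roll rotation tilts the nose up to a capped angle.
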(event EventBeginPlay)

(event Collision|EventActorBeginOverlap
  (params (OtherActor :type Actor%20Object%20Reference)))

(event EventTick
  (params (DeltaSeconds :type Float%20%28single-precision%29))
  (bind _staticmesh (Variables|Default|GetStaticMesh))
  (bind _endofrunwayx (Variables|Default|GetEndOfRunwayX))
  (bind _staticmesh_2 (Variables|Default|GetStaticMesh))
  (bind _returnvalue (Transformation|GetWorldLocation _staticmesh))
  (bind _returnvalue_2 (Math|Float|Absolute(Float) _endofrunwayx))
  (bind _returnvalue_3 (- _returnvalue_2 (.x _returnvalue)))
  (bind _returnvalue_4 (/ _returnvalue_3 -5.0))
  (bind _returnvalue_5 (* DeltaSeconds _returnvalue_4))
  (Effects|SpawnEmitteratLocation "/Game/Effects/Particles/Explosion/P_AsteroidExplosion.P_AsteroidExplosion" (Transformation|GetWorldLocation (Variables|Default|GetEnginePosition)) "0, 0, 0" "0.100000,0.100000,0.100000")
  (Transformation|AddActorWorldOffset (Math|Vector|MakeVector _returnvalue_5 _returnvalue_5 0.0) true)
  (if (<= (.x _returnvalue) 1e+03)
    (if (Variables|Default|GetOnlyOnce)
      ;[1 1 1] Make the glider pitch when it gains height
      (if (> (* 15 (- (Utilities|Time|GetGameTimeinSeconds) (Variables|Default|GetFirstGameTimeOfLiftOff))) 4e+01)
        (Transformation|SetRelativeRotation _staticmesh_2 (Math|Rotator|MakeRotator 3.2e+02 0.0 0.0) false false)
        (else
          (Transformation|SetRelativeRotation _staticmesh_2 (Math|Rotator|MakeRotator (- 3.6e+02 (* 15 (- (Utilities|Time|GetGameTimeinSeconds) (Variables|Default|GetFirstGameTimeOfLiftOff)))) 0.0 0.0) false false)))
      (Transformation|AddActorWorldOffset (Math|Vector|MakeVector 0.0 0.0 (* DeltaSeconds (Variables|Default|GetSpeed))) true)
      (else
        (Variables|Default|SetOnlyOnce true)
        (Variables|Default|SetFirstGameTimeOfLiftOff (Utilities|Time|GetGameTimeinSeconds))))))

(fn ConstructionScript)