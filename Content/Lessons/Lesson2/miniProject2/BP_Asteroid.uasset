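; BP_Asteroid is an asteroid actor that drifts through the level and explodes on overlap.
; On BeginPlay it picks a random unit vector as its moving direction.
; Tick moves it along that direction by Speed scaled by delta time, using a swept world offset.
; When its static mesh begins an overlap, it spawns an explosion emitter and sound at its location, then destroys itself.
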(event OnComponentBeginOverlap(StaticMesh)
  (params (OverlappedComponent :type Primitive%20Component%20Object%20Reference) (OtherActor :type Actor%20Object%20Reference) (OtherComp :type Primitive%20Component%20Object%20Reference) (OtherBodyIndex :type Integer) (bFromSweep :type Boolean) (SweepResult :type Hit%20Result%20Structure%20%28by%20ref%29))
  (bind _returnvalue (Transformation|GetActorLocation))
  (Effects|SpawnEmitteratLocation "/Game/Effects/Particles/Explosion/P_AsteroidExplosion.P_AsteroidExplosion" _returnvalue)
  (Audio|PlaySoundatLocation "/Game/Audio/SoundWaves/Effect/SW_Explosion_1.SW_Explosion_1" _returnvalue "0, 0, 0" 1.0 1.0 0.0 0 0 0)
  (Actor|DestroyActor))

(event EventBeginPlay
  ;[1 1 1] A random direction for every asteroid is set before it starts moving
  (Variables|Default|SetMovingDirection (Math|Random|RandomUnitVector)))

(event Collision|EventActorBeginOverlap
  (params (OtherActor :type Actor%20Object%20Reference)))

(event EventTick
  (params (DeltaSeconds :type Float%20%28single-precision%29))
  (Transformation|AddActorWorldOffset (* (Variables|Default|GetMovingDirection) (* DeltaSeconds (Variables|Default|GetSpeed))) true))

(fn ConstructionScript)