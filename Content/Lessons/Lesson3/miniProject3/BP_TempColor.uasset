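; BP_TempColor is a colored sphere that passes its color to any BP_PlainCube it hits, playing a sound at the cube.
; Construction creates a dynamic material, and UpdateColor stores a bucket color and applies it to that material.
; On its first non-cube hit near ground height, the BouncyColor timeline drives upward force on the sphere to keep it bouncing, guarded to start only once.
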(event Collision|EventHit
  (params (MyComp :type Primitive%20Component%20Object%20Reference) (Other :type Actor%20Object%20Reference) (OtherComp :type Primitive%20Component%20Object%20Reference) (bSelfMoved :type Boolean) (HitLocation :type Vector :default "0, 0, 0") (HitNormal :type Vector :default "0, 0, 0") (NormalImpulse :type Vector :default "0, 0, 0") (Hit :type Hit%20Result%20Structure%20%28by%20ref%29))
  (bind _asbp_plain_cube (Utilities|Casting|CastToBP_PlainCube Other)
    (:then
      (Audio|PlaySoundatLocation "/Game/Audio/SoundWaves/Effect/SW_Jump_3.SW_Jump_3" (Transformation|GetActorLocation Other) "0, 0, 0" 1.0 1.0 0.0 0 0 0)
      (Default|UpdateColor _asbp_plain_cube (Variables|Default|GetCurrentColor)))
    (:CastFailed
      ;[1 1 1] If a color hits the ground, it will continue bouncing by adding force according to a timeline
      (if (<= (.z HitLocation) 0.05)
        (if (not (Variables|Default|GetHaveBounced))
          (Variables|Default|SetHaveBounced true)
          (Variables|Default|SetOrigin (Transformation|GetActorLocation))
          (bind _data (Timeline|BouncyColor PlayFromStart)
            (:Update
              (Physics|AddForce (Variables|Default|GetSphere) (* "0.000000,0.000000,27000.000000" _data) "None" false))))))))

(fn ConstructionScript
  (bind _returnvalue (Rendering|Material|CreateDynamicMaterialInstance (Variables|Default|GetSphere) 0 0 "None" :!class /Script/Engine.PrimitiveComponent))
  (Variables|Default|SetSphereColor _returnvalue))

(fn UpdateColor
  (params (Bucket%20color :type Linear%20Color%20Structure))
  (bind _output_get (Variables|Default|SetCurrentColor Bucket%20color))
  (Rendering|Material|SetVectorParameterValue (Variables|Default|GetSphereColor) "Color" _output_get :!class /Script/Engine.MaterialInstanceDynamic))