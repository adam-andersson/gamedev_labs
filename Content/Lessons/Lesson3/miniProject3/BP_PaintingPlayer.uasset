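; Player Blueprint for a painting mini-project that lets the user drag physics objects with a camera-aimed crosshair and left mouse button.
; Visibility traces along the camera's forward vector position the crosshair and drive a PhysicsHandle for grabbing and moving.
; Clicking non-physics button actors spawns plain cubes; clicking buckets replaces them with color spheres of the same color.
; One second after release, a dragged color sphere explodes unless dragging has resumed.
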(event EventTick
  (params (DeltaSeconds :type Float%20%28single-precision%29))
  (CallFunction|UpdateDrag)
  ;[1 1 1] Update crosshair/reticle location
  (bind (_location _forward_vector) (CallFunction|GetPlayerVRCameraProperties))
  (bind (_outhit _returnvalue) (Collision|LineTraceByChannel _location (+ _location (* _forward_vector 1e+04)) "TraceTypeQuery1" false 0 "None"))
  (if _returnvalue
    (Transformation|SetWorldLocation (Variables|Default|GetCrosshair) (.Location (Collision|BreakHitResult _outhit)) false false)
    (else
      (Transformation|SetWorldLocation (Variables|Default|GetCrosshair) (+ _location (* _forward_vector 1e+04)) false false))))

(event Input|MouseEvents|LeftMouseButton
  (params (Key :type Key%20Structure :default "None"))
  (bind _draggedhit (Variables|Default|GetDraggedHit))
  (bind (_bblockinghit _binitialoverlap _time _distance _location _impactpoint _normal _impactnormal _physmat _hitactor _hitcomponent) (Collision|BreakHitResult _draggedhit))
  (bind _returnvalue (Transformation|GetWorldLocation _hitcomponent))
  (:Pressed
    (CallFunction|StartDrag))
  (:Released
    (CallFunction|EndDrag)
    ;[1 1 1] Destroys (and spawns sound and emitter) 1 seconds after dragging a color sphere
    (Utilities|FlowControl|Delay 1.0)
    (if (not (Variables|Default|GetisDragging))
      (bind _asbp_temp_color (Utilities|Casting|CastToBP_TempColor _hitactor))
      (Effects|SpawnEmitteratLocation "/Game/Effects/Particles/Explosion/P_NeonExplosion.P_NeonExplosion" _returnvalue)
      (Audio|PlaySoundatLocation "/Game/Audio/SoundWaves/Effect/SW_Explosion_1.SW_Explosion_1" _returnvalue "0, 0, 0" 1.0 1.0 0.0 0 0 0)
      (Actor|DestroyActor _asbp_temp_color))))

(fn ConstructionScript)

(fn StartDrag
  (if (not (Variables|Default|GetisDragging))
    (bind (_location _forward_vector) (CallFunction|GetPlayerVRCameraProperties))
    (bind (_outhit _returnvalue) (Collision|LineTraceByChannel _location (+ _location (* _forward_vector 1e+04)) "TraceTypeQuery1" false 0 "None"))
    (if _returnvalue
      (bind _output_get (Variables|Default|SetDraggedHit _outhit))
      (if (Physics|IsSimulatingPhysics (.HitComponent (Collision|BreakHitResult _output_get)) "None")
        (Class|PhysicsHandleComponent|GrabComponentatLocation (Variables|Default|GetPhysicsHandle) (.HitComponent (Collision|BreakHitResult _output_get)) "None" (Transformation|GetWorldLocation (.HitComponent (Collision|BreakHitResult _output_get))))
        (Variables|Default|SetisDragging true)
        (else
          ;[1 1 1] If we click on an actor that's not simulating physics, we check if it is a 'button' and if so call the function to spawn a new block
          (Utilities|Casting|CastToBP_ButtonForCube (.HitActor (Collision|BreakHitResult _output_get))
            (:then
              (CallFunction|SpawnBlock (Transformation|GetWorldLocation (.HitComponent (Collision|BreakHitResult _output_get)))))
            (:CastFailed
              ;[1 1 1] If it's not a 'button' we check if it is a 'bucket', and if call the funcion to spawn a color sphere
              (bind _asbp_color_bucket (Utilities|Casting|CastToBP_ColorBucket (.HitActor (Collision|BreakHitResult _output_get))))
              (CallFunction|SpawnTempColor (Transformation|GetWorldLocation (.HitComponent (Collision|BreakHitResult _output_get))) _asbp_color_bucket))))))))

(fn EndDrag
  (Utilities|IsValid (Class|PhysicsHandleComponent|GetGrabbedComponent (Variables|Default|GetPhysicsHandle))
    (:Is%20Valid
      (Physics|Components|PhysicsHandle|ReleaseComponent (Variables|Default|GetPhysicsHandle))
      (Variables|Default|SetisDragging false))))

(fn UpdateDrag
  (if (Variables|Default|GetisDragging)
    (bind (_location _forward_vector) (CallFunction|GetPlayerVRCameraProperties))
    (bind _outhit (Collision|LineTraceByChannel _location (+ _location (* _forward_vector 1e+04)) "TraceTypeQuery1" false 0 "None"))
    (Physics|Components|PhysicsHandle|SetTargetLocation (Variables|Default|GetPhysicsHandle) (.Location (Collision|BreakHitResult _outhit)))))

(fn SpawnBlock
  (params (ActorLocation :type Vector))
  (Game|SpawnActorfromClass "/Game/Lessons/Lesson3/miniProject3/BP_PlainCube.BP_PlainCube_C" (Math|Conversions|ToTransform(Vector) (- ActorLocation "100.000000, 0, 0")) "Undefined" 0 0))

(fn SpawnTempColor
  (params (Location :type Vector) (Actor :type Actor%20Object%20Reference))
  (bind _asbp_color_bucket (Utilities|Casting|CastToBP_ColorBucket Actor))
  (bind _returnvalue (Game|SpawnActorfromClass "/Game/Lessons/Lesson3/miniProject3/BP_TempColor.BP_TempColor_C" (Math|Conversions|ToTransform(Vector) (- Location "0.000000,0.000000,-35.000000")) "Undefined" 0 0))
  (Default|UpdateColor _returnvalue (Variables|/Game/Lessons/Lesson3/miniProject3/BP_ColorBucket.BP_ColorBucket_C|GetRetrieveColorVector _asbp_color_bucket))
  (Actor|DestroyActor _asbp_color_bucket))