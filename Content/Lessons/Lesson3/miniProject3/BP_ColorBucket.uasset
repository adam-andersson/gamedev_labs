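; Color bucket actor that takes a random color on spawn and destroys itself about 30 seconds later.
; A timeline scales each RGB channel, applies a 2.19 gamma exponent and writes the result to the mesh's dynamic material, created in the construction script.
; On overlapping another color bucket it destroys that one, intended to replace an older bucket at the same spawn location.
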(event EventBeginPlay
  (Variables|Default|SetRandomStartColor (Math|Vector|MakeVector (Math|Random|RandomFloatinRange 0.0 1.0) (Math|Random|RandomFloatinRange 0.0 1.0) (Math|Random|RandomFloatinRange 0.0 1.0)))
  (bind (_direction _multiplier_r _multiplier_g _multiplier_b) (Timeline|FadeColors PlayFromStart)
    (:Update
      (bind _output_get (Variables|Default|SetRetrieveColorVector (Utilities|Struct|MakeLinearColor (Math|Float|Power (* (.x (Variables|Default|GetRandomStartColor)) _multiplier_r) 2.19) (Math|Float|Power (* (.y (Variables|Default|GetRandomStartColor)) _multiplier_g) 2.19) (Math|Float|Power (* (.z (Variables|Default|GetRandomStartColor)) _multiplier_b) 2.19) 0.6)))
      (Rendering|Material|SetVectorParameterValue (Variables|Default|GetBucketColor) "Color" _output_get :!class /Script/Engine.MaterialInstanceDynamic)
      (Utilities|FlowControl|Delay 3e+01)
      (Actor|DestroyActor))))

(event Collision|EventActorBeginOverlap
  (params (OtherActor :type Actor%20Object%20Reference))
  ;[1 1 1] If we spawn a bucket at the same location as another bucket,we delete the first one.
  (bind _asbp_color_bucket (Utilities|Casting|CastToBP_ColorBucket OtherActor))
  (Actor|DestroyActor _asbp_color_bucket))

(fn ConstructionScript
  (bind _returnvalue (Rendering|Material|CreateDynamicMaterialInstance (Variables|Default|GetBucketMesh) 0 0 "None" :!class /Script/Engine.PrimitiveComponent))
  (Variables|Default|SetBucketColor _returnvalue))